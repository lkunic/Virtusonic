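; Bass instrument actor that spawns its sound sources and picks on BeginPlay.
; Audio sources are stacked vertically, each given an indexed bass sound and frequency, and registered with the AudioController.
; Picks are spaced sideways, given the bass pick mesh, and registered with the PickController.
; Both sets attach to this actor's owner rather than itself; SpawnFretFingers is an empty stub.
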(event EventBeginPlay
  (CallFunction|SpawnAudioSources)
  (CallFunction|SpawnPicks))

(event Collision|EventActorBeginOverlap
  (params (OtherActor :type Actor%20Object%20Reference)))

(event EventTick
  (params (DeltaSeconds :type Float%20%28single-precision%29)))

(fn ConstructionScript)

(fn SpawnAudioSources
  (for _index (range 0 4)
    (bind _returnvalue (Game|SpawnActorfromClass "/Script/Virtusonic.AudioSource" (Math|Transform|MakeTransform (Math|Vector|MakeVector 5.0 0.0 (+ 105.0 (* (Math|Conversions|ToFloat(Integer) _index) -2.5)))) "Undefined" self 0))
    (bind _output_get (Variables|Default|SetAudioSource _returnvalue))
    (Transformation|AttachActorToActor _output_get (Components|GetOwner) "None" "KeepRelative" "KeepRelative" "KeepRelative" true)
    (Class|AudioController|AddAudioSource (Variables|Default|GetAudioController) (Variables|Default|GetAudioSource))
    (Class|AudioSource|SetSound (Variables|Default|GetAudioSource) (Utilities|Array|Get(acopy) (Variables|Bass|GetBassSounds) _index) (Utilities|Array|Get(acopy) (Variables|Bass|GetBassSoundFrequencies) _index))))

(fn SpawnPicks
  (for _index (range 0 4)
    (bind _returnvalue (Game|SpawnActorfromClass "/Script/Virtusonic.Pick" (Math|Transform|MakeTransform (Math|Vector|MakeVector 0.0 (* (Math|Conversions|ToFloat(Integer) _index) -2.0) 1e+02)) "Undefined" self 0))
    (bind _output_get (Variables|Default|SetPick _returnvalue))
    (Class|SkinnedMeshComponent|SetSkeletalMesh (Variables|/Script/Engine.SkeletalMeshActor|GetSkeletalMeshComponent _output_get) "/Game/Models/Bass/Pick/BassPick.BassPick" true)
    (Transformation|AttachActorToActor (Variables|Default|GetPick) (Components|GetOwner) "None" "KeepRelative" "KeepRelative" "KeepRelative" true)
    (Class|PickController|AddPick (Variables|Default|GetPickController) (Variables|Default|GetPick))))

(fn SpawnFretFingers)